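; Main hall grid actor for the art heist game, with a trigger box that decides the match result when a robber enters it.
; A player Robber pauses the game mode and sets the finish UI text to won or lost, based on whether its stolen percent exceeds a small threshold.
; An AI robber entering instead makes the player's Guard lose.
; The construction script calls SetGameMode and passes the Cube to SetBox.
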(event `self.Box.OnComponentBeginOverlap`
  (params (OverlappedComponent :type "PrimitiveComponent Object Reference") (OtherActor :type "Actor Object Reference") (OtherComp :type "PrimitiveComponent Object Reference") (OtherBodyIndex :type Integer) (bFromSweep :type Boolean) (SweepResult :type "HitResult Structure (by ref)"))
  (if (`self.ActorHasTag` OtherActor "Playable")
    (if (`self.ActorHasTag` OtherActor "Robber")
      (bind _asbp_art_guard_game_mode (cast `/Game/ThirdPersonBP/BP_ArtGuardGameMode` (`GameplayStatics.GetGameMode`)))
      (bind _asbp_robber (cast `/Game/ThirdPersonBP/Blueprints/BP_Robber` OtherActor))
      (`/Game/ThirdPersonBP/BP_ArtGuardGameMode.Pause` _asbp_art_guard_game_mode)
      (bind _percent (`/Game/ThirdPersonBP/Blueprints/BP_Robber.GetStolenPercent` _asbp_robber))
      (if (> _percent 0.01)
        (set `self.WInLose` "YOU WON")
        (else
          (set `self.WInLose` "YOU LOST")))
      (set `/Game/UI/EndGameUI/FinishUI.ResultText` (`self.WInLose`) (`/Game/ThirdPersonBP/BP_ArtGuardGameMode.UIFinish` _asbp_art_guard_game_mode))
      (elif (`self.ActorHasTag` OtherActor "RobberAI")
        (bind _asbp_guard (cast `/Game/ThirdPersonBP/Blueprints/BP_Guard` (`GameplayStatics.GetPlayerCharacter` 0)))
        (`/Game/ThirdPersonBP/Blueprints/BP_Guard.Lose` _asbp_guard)))))

(fn `UserConstructionScript`
  (`self.SetGameMode`)
  (`self.SetBox` (`self.Cube`)))