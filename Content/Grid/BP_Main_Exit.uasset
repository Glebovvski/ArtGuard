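; Main level exit for the art heist game that resolves the round when a Playable-tagged actor overlaps its box.
; A Robber sets a win or loss from its stolen percentage, updating the game mode's finish UI and pausing.
; A RobberAI triggers the player guard's Lose if carrying stolen pictures, otherwise Catch; a Guard entering also loses.
; A helper toggles the exit icon's visibility.
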(event `self.Box.OnComponentBeginOverlap`
  (params (OverlappedComponent :type "PrimitiveComponent Object Reference") (OtherActor :type "Actor Object Reference") (OtherComp :type "PrimitiveComponent Object Reference") (OtherBodyIndex :type Integer) (bFromSweep :type Boolean) (SweepResult :type "HitResult Structure (by ref)"))
  (bind _returnvalue (`GameplayStatics.GetPlayerCharacter` 0))
  (if (`self.ActorHasTag` OtherActor "Playable")
    (if (`self.ActorHasTag` OtherActor "Robber")
      (bind _asbp_art_guard_game_mode (cast `/Game/ThirdPersonBP/BP_ArtGuardGameMode` (`GameplayStatics.GetGameMode`)))
      (bind _asbp_robber (cast `/Game/ThirdPersonBP/Blueprints/BP_Robber` OtherActor))
      (bind _percent (`/Game/ThirdPersonBP/Blueprints/BP_Robber.GetStolenPercent` _asbp_robber))
      (bind _returnvalue_2 (> _percent 0.01))
      (if _returnvalue_2
        (set `self.WInLose` "YOU WON")
        (else
          (set `self.WInLose` "YOU LOST")))
      (set `/Game/UI/FinishUI/FinishUI.ResultText` (`self.WInLose`) (`/Game/ThirdPersonBP/BP_ArtGuardGameMode.UIFinish` _asbp_art_guard_game_mode))
      (`/Game/ThirdPersonBP/BP_ArtGuardGameMode.Pause` _asbp_art_guard_game_mode)
      (set `/Game/ThirdPersonBP/BP_ArtGuardGameMode.Won` _returnvalue_2 _asbp_art_guard_game_mode)
      (elif (`self.ActorHasTag` OtherActor "RobberAI")
        (bind _asbp_robber_ai (cast `/Game/ThirdPersonBP/Blueprints/BP_RobberAI` OtherActor))
        (bind _returnvalue_3 (`Robber.GetPicturesStolen` _asbp_robber_ai))
        (if (> _returnvalue_3 0)
          (bind _asbp_guard (cast `/Game/ThirdPersonBP/Blueprints/BP_Guard` _returnvalue :!label _label))
          (`/Game/ThirdPersonBP/Blueprints/BP_Guard.Lose` _asbp_guard)
          (else
            (bind _asbp_guard_2 (cast `/Game/ThirdPersonBP/Blueprints/BP_Guard` _returnvalue))
            (`Guard.Catch` _asbp_guard_2)))
        (elif (`self.ActorHasTag` OtherActor "Guard")
          (goto _label))))))

(fn `Set Exit Visibility`
  (params (Visibility :type "ESlateVisibility Enum" :default "Visible"))
  (`/Game/UI/UI_Icon/ActorIcon_Component.Set Icon Visibility` (`self.ExitIcon`) Visibility))

(fn `UserConstructionScript`
  (`self.SetGameMode`)
  (`self.SetBox` (`self.Cube`)))