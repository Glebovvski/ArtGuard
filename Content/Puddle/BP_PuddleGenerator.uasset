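; BP_PuddleGenerator spawns a cluster of eight randomly scaled puddles around itself and slows characters that enter the area.
; BeginPlay scatters BP_Puddle actors, then scales a trigger Box by MaxSize, which comes from separate random rolls rather than the spawned scales.
; Overlapping components tagged "Puddle" trigger a walk-speed cap, with the original speed stashed in MaxCustomMovementSpeed and restored on exit.
; Array and average-size logic is left disconnected.
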(event `self.ReceiveBeginPlay`
  (bind _returnvalue (`KismetMathLibrary.RandomFloatInRange` 1.0 5.0))
  (bind _maxsize (`self.MaxSize`))
  (for _ (range 8)
    (bind (_x _y _z) (`self.GetRandomLocation`))
    (bind _returnvalue_2 (`|SpawnActorFromClass` "/Game/Puddle/BP_Puddle.BP_Puddle_C" (`KismetMathLibrary.MakeTransform` (`KismetMathLibrary.MakeVector` _x _y _z) (struct) (`KismetMathLibrary.MakeVector` _returnvalue _returnvalue 1.0)) "Undefined" "OverrideRootScale" null null))
    (if (> _returnvalue (`self.MaxSize`))
      (set `self.MaxSize` _returnvalue)))
  (`SceneComponent.SetWorldScale3D` (`self.Box`) (`KismetMathLibrary.MakeVector` _maxsize _maxsize 10.0)))

(event `self.Box.OnComponentBeginOverlap`
  (params (OverlappedComponent :type "PrimitiveComponent Object Reference") (OtherActor :type "Actor Object Reference") (OtherComp :type "PrimitiveComponent Object Reference") (OtherBodyIndex :type Integer) (bFromSweep :type Boolean) (SweepResult :type "HitResult Structure (by ref)"))
  (bind _returnvalue (`self.GetComponentByClass` OtherActor "/Script/Engine.CharacterMovementComponent"))
  (if (`ActorComponent.ComponentHasTag` OtherComp "Puddle")
    (set `CharacterMovementComponent.MaxCustomMovementSpeed` (`CharacterMovementComponent.MaxWalkSpeed` _returnvalue) _returnvalue)
    (set `CharacterMovementComponent.MaxWalkSpeed` 300.0 _returnvalue)))

(event `self.Box.OnComponentEndOverlap`
  (params (OverlappedComponent :type "PrimitiveComponent Object Reference") (OtherActor :type "Actor Object Reference") (OtherComp :type "PrimitiveComponent Object Reference") (OtherBodyIndex :type Integer))
  (bind _returnvalue (`self.GetComponentByClass` OtherActor "/Script/Engine.CharacterMovementComponent"))
  (if (`ActorComponent.ComponentHasTag` OtherComp "Puddle")
    (set `CharacterMovementComponent.MaxWalkSpeed` (`CharacterMovementComponent.MaxCustomMovementSpeed` _returnvalue) _returnvalue)))

(fn `GetRandomLocation`
  (returns (X :type "Float (double-precision)") (Y :type "Float (double-precision)") (Z :type "Float (double-precision)"))
  (bind (_returnvalue_x _returnvalue_y _returnvalue_z) (`KismetMathLibrary.BreakVector` (`self.K2_GetActorLocation`)))
  (return (+ (`KismetMathLibrary.RandomFloatInRange` -50.0 50.0) _returnvalue_x) (+ (`KismetMathLibrary.RandomFloatInRange` -50.0 50.0) _returnvalue_y) _returnvalue_z))

(fn `UserConstructionScript`)