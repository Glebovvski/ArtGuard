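; BP_Room1 is a room actor that sets up its floor, arrows, walls and exits.
; The construction script passes Plane1 as the floor and calls SetGameMode.
; On BeginPlay it hands the children of its MainArrows, LeftArrows and RightArrows components to SetArrows, then calls SpawnWalls and SpawnExits.
; The logic behind these calls is defined outside this graph, and Tick and overlap events are unused.
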(event `self.ReceiveBeginPlay`
  (`self.SetArrows` (`SceneComponent.GetChildrenComponents` (`self.MainArrows`) false) (`SceneComponent.GetChildrenComponents` (`self.LeftArrows`) false) (`SceneComponent.GetChildrenComponents` (`self.RightArrows`) false))
  (`self.SpawnWalls`)
  (`self.SpawnExits`))

(fn `UserConstructionScript`
  (`self.SetFloor` (`self.Plane1`))
  (`self.SetGameMode`))