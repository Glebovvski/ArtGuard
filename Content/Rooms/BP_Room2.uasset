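; BP_Room2 is a room actor that builds its walls and exits when play begins.
; Its construction script registers a Plane as the floor and calls SetGameMode.
; On BeginPlay it passes the children of the MainArrows, LeftArrows and RightArrows components to SetupRoom, which stores them through SetArrows, then runs SpawnWalls and SpawnExits, whose logic lives outside these graphs.
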(event `self.ReceiveBeginPlay`
  (`self.SetupRoom` (`SceneComponent.GetChildrenComponents` (`self.MainArrows`) false) (`SceneComponent.GetChildrenComponents` (`self.LeftArrows`) false) (`SceneComponent.GetChildrenComponents` (`self.RightArrows`) false)))

(fn `SetupRoom`
  (params (MainArrowsToSet :type "Array of SceneComponent Object Reference") (LeftArrowsToSet :type "Array of SceneComponent Object Reference") (RightArrowsToSet :type "Array of SceneComponent Object Reference"))
  (`self.SetArrows` MainArrowsToSet LeftArrowsToSet RightArrowsToSet)
  (`self.SpawnWalls`)
  (`self.SpawnExits`))

(fn `UserConstructionScript`
  (`self.SetFloor` (`self.Plane`))
  (`self.SetGameMode`))