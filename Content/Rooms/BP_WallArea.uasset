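; BP_WallArea is a room wall piece that can dress itself with a framed picture.
; The construction script passes its WallBP component to SetWallProperties, which is defined outside this file.
; SpawnFullWall repeats that setup, spawns a frame at zero location and rotation with the fence hidden, then calls SpawnPicture on it.
; The event graph is inactive, holding only unreachable logic that feeds wall scale into material parameters.
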(event `self.ReceiveTick`
  (params (DeltaSeconds :type "Float (single-precision)")))

(fn `SpawnFullWall`
  (`self.SetWallProperties` (`self.Wall_BP`))
  (bind _returnvalue (`self.SpawnFrame` (0.0 0.0 0.0)))
  (`Frame.SpawnPicture` _returnvalue true))

(fn `UserConstructionScript`
  (`self.SetWallProperties` (`self.Wall_BP`)))