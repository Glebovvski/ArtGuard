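; BP_Room5 is a room Blueprint that configures its floor, directional collision boxes and arrow markers through shared room functions.
; The construction script sets Plane1 as the floor and calls SetGameMode.
; On BeginPlay it registers the four collision boxes, then passes the child components of four arrow groups to SetupRoom.
; SetupRoom only forwards them to SetArrows, leaving its SpawnExits and SpawnWalls calls disconnected.
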(event `self.ReceiveBeginPlay`
  (`self.SetupCollisionBoxes` (`self.UpCollision`) (`self.DownCollision`) (`self.RightCollision`) (`self.LeftCollision`))
  (`self.SetupRoom` (`SceneComponent.GetChildrenComponents` (`self.UpArrows`) false) (`SceneComponent.GetChildrenComponents` (`self.BottomArrows`) false) (`SceneComponent.GetChildrenComponents` (`self.LeftArrows`) false) (`SceneComponent.GetChildrenComponents` (`self.RightArrows`) false)))

(fn `SetupRoom`
  (params (UpMainArrowsToSet :type "Array of SceneComponent Object Reference") (BottomMainArrowsToSet :type "Array of SceneComponent Object Reference") (LeftArrowsToSet :type "Array of SceneComponent Object Reference") (RightArrowsToSet :type "Array of SceneComponent Object Reference"))
  (`self.SetArrows` UpMainArrowsToSet BottomMainArrowsToSet LeftArrowsToSet RightArrowsToSet))

(fn `UserConstructionScript`
  (`self.SetFloor` (`self.Plane1`))
  (`self.SetGameMode`))