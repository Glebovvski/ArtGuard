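; BP_Picture is a stealable picture that shows the robber a risk percentage when they come near it.
; Overlapping the risk collision runs AssessRisk, which checks CanSteal and the Robber tag, then fills the RiskUI widget with the robber's risk value and color.
; Leaving the collision hides that widget.
; The construction script sets the plane, and the first Tick applies the fence's visibility flag.
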(event `self.ReceiveBeginPlay`)

(event `self.ReceiveTick`
  (params (DeltaSeconds :type "Float (single-precision)"))
  (`/Engine/EditorBlueprintResources/StandardMacros.DoOnce` false
    (:`Completed`
      (`SceneComponent.SetVisibility` (`self.Fence`) (`self.IsFenceVisible`) false))))

(event `self.RiskCollision.OnComponentBeginOverlap`
  (params (OverlappedComponent :type "PrimitiveComponent Object Reference") (OtherActor :type "Actor Object Reference") (OtherComp :type "PrimitiveComponent Object Reference") (OtherBodyIndex :type Integer) (bFromSweep :type Boolean) (SweepResult :type "HitResult Structure (by ref)"))
  (`self.Assess Risk` OtherComp OtherActor))

(event `self.RiskCollision.OnComponentEndOverlap`
  (params (OverlappedComponent :type "PrimitiveComponent Object Reference") (OtherActor :type "Actor Object Reference") (OtherComp :type "PrimitiveComponent Object Reference") (OtherBodyIndex :type Integer))
  (if (`ActorComponent.IsBeingDestroyed` (`self.RiskText`))
    _
    (elif (`ActorComponent.ComponentHasTag` OtherComp "Robber")
      (bind _asrisk_ui (cast `/Game/UI/RiskAssessmnetUI/RiskUI` (`WidgetComponent.GetUserWidgetObject` (`self.RiskText`))))
      (set `/Game/UI/RiskAssessmnetUI/RiskUI.RiskVisibility` "Hidden" _asrisk_ui))))

(fn `Assess Risk`
  (params (`Other Comp` :type "ActorComponent Object Reference") (Robber :type "Object Object Reference"))
  (bind _returnvalue (`self.CanSteal`))
  (if _returnvalue
    (if (`ActorComponent.ComponentHasTag` `Other Comp` "Robber")
      (bind _asbp_robber (cast `/Game/ThirdPersonBP/Blueprints/BP_Robber` Robber))
      (bind _returnvalue_2 (`Robber.GetRiskAssessment` _asbp_robber))
      (bind _returnvalue_3 (`KismetMathLibrary.FTrunc` _returnvalue_2))
      (bind _returnvalue_4 (`Robber.GetColorOfRisk` _asbp_robber _returnvalue_3))
      (bind _asrisk_ui (cast `/Game/UI/RiskAssessmnetUI/RiskUI` (`WidgetComponent.GetUserWidgetObject` (`self.RiskText`))))
      (`UserWidget.SetColorAndOpacity` _asrisk_ui (`KismetMathLibrary.Conv_ColorToLinearColor` _returnvalue_4))
      (set `/Game/UI/RiskAssessmnetUI/RiskUI.RiskVisibility` "Visible" _asrisk_ui)
      (set `/Game/UI/RiskAssessmnetUI/RiskUI.RiskText` (`KismetTextLibrary.Conv_StringToText` (`KismetStringLibrary.Concat_StrStr` "RISK: " (`KismetStringLibrary.Conv_IntToString` _returnvalue_3) "%")) _asrisk_ui))))

(fn `UserConstructionScript`
  (`self.SetPlane` (`self.Plane2`)))